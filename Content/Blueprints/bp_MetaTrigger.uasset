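; bp_MetaTrigger is a level finish trigger that advances the game once all BP_Crystal actors are gone.
; Any overlap with its box runs CrystalCheck, which only prints a message while crystals remain; the player-pawn check is unused.
; Otherwise Complitelevel finds the current level name in ArrayLevels and opens the next entry, or quits the game on the last one.
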(event `self.box_collision.OnComponentBeginOverlap`
  (params (OverlappedComponent :type "PrimitiveComponent Object Reference") (OtherActor :type "Actor Object Reference") (OtherComp :type "PrimitiveComponent Object Reference") (OtherBodyIndex :type Integer) (bFromSweep :type Boolean) (SweepResult :type "HitResult Structure (by ref)"))
  (if true
    (bind _returnvalue (`self.Crystal Check`))
    (if _returnvalue
      (`KismetSystemLibrary.PrintString` "GG")
      (else
        (`self.complitelevel`)))))

(fn `complitelevel`
  (if (`self.isitlastlevell`)
    (`KismetSystemLibrary.QuitGame` null "Quit")
    (else
      (`KismetSystemLibrary.PrintString` "hura! poziom pokonany")
      (`GameplayStatics.OpenLevel` (`self.newlevel`)))))

(fn `Crystal Check`
  (returns (ReturnValue :type Boolean))
  (bind _outactors (`GameplayStatics.GetAllActorsOfClass` "/Game/Blueprints/BP_Crystal.BP_Crystal_C"))
  (return (> (`KismetArrayLibrary.Array_Length` _outactors) 0)))

(fn `currentlvlindex`
  (returns (ReturnValue :type Integer))
  (bind _returnvalue (`GameplayStatics.GetCurrentLevelName` true))
  (return (`KismetArrayLibrary.Array_Find` (`self.array levels`) (`KismetStringLibrary.Conv_StringToName` _returnvalue))))

(fn `isitlastlevell`
  (returns (ReturnValue :type Boolean))
  (return (== (`self.currentlvlindex`) (`KismetArrayLibrary.Array_LastIndex` (`self.array levels`)))))

(fn `newlevel`
  (returns (Output :type Name))
  (return (`|GetArrayItem` (`self.array levels`) (+ (`self.currentlvlindex`) 1))))

(fn `UserConstructionScript`)